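; Master pickup actor for level-completion items, which can be a Key, Intel or Quest Item.
; When the third-person character overlaps the sphere, it highlights its meshes through custom depth, shows a widget and enables input, with a CanPick flag cleared on exit.
; Pressing ItemInteraction while CanPick is set increments the character counter matching the RandomItem type, then destroys the actor.
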(event `self.Sphere.OnComponentBeginOverlap`
  (params (OverlappedComponent :type "PrimitiveComponent Object Reference") (OtherActor :type "Actor Object Reference") (OtherComp :type "PrimitiveComponent Object Reference") (OtherBodyIndex :type Integer) (bFromSweep :type Boolean) (SweepResult :type "HitResult Structure (by ref)"))
  ;[0.6563 0.3219 1] Random Pickup items to complete the level
  (cast `/Game/ThirdPerson/Blueprints/SS_ThirdPersonCharacter` OtherActor)
  (`PrimitiveComponent.SetRenderCustomDepth` (`self.SkeletalMesh`) true)
  (`PrimitiveComponent.SetRenderCustomDepth` (`self.StaticMesh`) true)
  (`SceneComponent.SetVisibility` (`self.Widget`) true false)
  (set `self.canPick?` true)
  (`self.EnableInput` (`GameplayStatics.GetPlayerController` 0)))

(event `self.Sphere.OnComponentEndOverlap`
  (params (OverlappedComponent :type "PrimitiveComponent Object Reference") (OtherActor :type "Actor Object Reference") (OtherComp :type "PrimitiveComponent Object Reference") (OtherBodyIndex :type Integer))
  ;[0.6563 0.3219 1] Random Pickup items to complete the level
  (cast `/Game/ThirdPerson/Blueprints/SS_ThirdPersonCharacter` OtherActor)
  (`PrimitiveComponent.SetRenderCustomDepth` (`self.StaticMesh`) false)
  (`PrimitiveComponent.SetRenderCustomDepth` (`self.SkeletalMesh`) false)
  (`SceneComponent.SetVisibility` (`self.Widget`) false false)
  (set `self.canPick?` false))

(event `InputAction|ItemInteraction`
  (params (Key :type "Key Structure"))
  ;[0.6563 0.3219 1] Random Pickup items to complete the level
  (:`Pressed`
    (if (`self.canPick?`)
      (switch `/Game/RandomPickup/RandomPickupType` (`self.RandomItem`)
        (:`NewEnumerator1`
          (bind _asss_third_person_character (cast `/Game/ThirdPerson/Blueprints/SS_ThirdPersonCharacter` (`GameplayStatics.GetPlayerCharacter` 0)))
          (bind _result (`/Engine/EditorBlueprintResources/StandardMacros.IncrementInt` (`/Game/ThirdPerson/Blueprints/SS_ThirdPersonCharacter.key` _asss_third_person_character))
            (:`  `
              (set `/Game/ThirdPerson/Blueprints/SS_ThirdPersonCharacter.key` _result _asss_third_person_character)
              (`self.K2_DestroyActor`))))
        (:`NewEnumerator2`
          (bind _asss_third_person_character_2 (cast `/Game/ThirdPerson/Blueprints/SS_ThirdPersonCharacter` (`GameplayStatics.GetPlayerCharacter` 0)))
          (bind _result_2 (`/Engine/EditorBlueprintResources/StandardMacros.IncrementInt` (`/Game/ThirdPerson/Blueprints/SS_ThirdPersonCharacter.Intel` _asss_third_person_character_2))
            (:`  `
              (set `/Game/ThirdPerson/Blueprints/SS_ThirdPersonCharacter.Intel` _result_2 _asss_third_person_character_2)
              (`self.K2_DestroyActor`))))
        (:`NewEnumerator3`
          (bind _asss_third_person_character_3 (cast `/Game/ThirdPerson/Blueprints/SS_ThirdPersonCharacter` (`GameplayStatics.GetPlayerCharacter` 0)))
          (bind _result_3 (`/Engine/EditorBlueprintResources/StandardMacros.IncrementInt` (`/Game/ThirdPerson/Blueprints/SS_ThirdPersonCharacter.QuestItem` _asss_third_person_character_3))
            (:`  `
              (set `/Game/ThirdPerson/Blueprints/SS_ThirdPersonCharacter.QuestItem` _result_3 _asss_third_person_character_3)
              (`self.K2_DestroyActor`))))))))

(fn `UserConstructionScript`)