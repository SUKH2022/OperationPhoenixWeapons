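; Door Blueprint that prompts the player to open it with a key, or to find one first.
; A box overlap toggles custom depth on the mesh and a Door_UI widget, whose text depends on the character's Key count.
; Having a key enables input and sets CanDoorOpen, which the ItemInteraction press checks.
; That branch is empty and the OpenDoor node is unconnected, so the door never actually opens.
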(event `self.Box.OnComponentBeginOverlap`
  (params (OverlappedComponent :type "PrimitiveComponent Object Reference") (OtherActor :type "Actor Object Reference") (OtherComp :type "PrimitiveComponent Object Reference") (OtherBodyIndex :type Integer) (bFromSweep :type Boolean) (SweepResult :type "HitResult Structure (by ref)"))
  ;[0.3883 0.9622 1] Door logic to open with key and find it to open
  (bind _asss_third_person_character (cast `/Game/ThirdPerson/Blueprints/SS_ThirdPersonCharacter` OtherActor))
  (set `self.SSRef` _asss_third_person_character)
  (`PrimitiveComponent.SetRenderCustomDepth` (`self.StaticMesh`) true)
  (`SceneComponent.SetVisibility` (`self.Widget`) true false)
  (if (>= (`/Game/ThirdPerson/Blueprints/SS_ThirdPersonCharacter.key` (`self.SSRef`)) 1)
    (bind _asdoor_ui (cast `/Game/Door_BP/Door_UI` (`WidgetComponent.GetUserWidgetObject` (`self.Widget`))))
    (set `/Game/Door_BP/Door_UI.KeyText` "Open Door [F]" _asdoor_ui)
    (`self.EnableInput` (`GameplayStatics.GetPlayerController` 0))
    (set `self.canDoorOpen?` true)
    (else
      (bind _asdoor_ui_2 (cast `/Game/Door_BP/Door_UI` (`WidgetComponent.GetUserWidgetObject` (`self.Widget`))))
      (set `/Game/Door_BP/Door_UI.KeyText` "Find Key to Open Door" _asdoor_ui_2)
      (set `self.canDoorOpen?` false))))

(event `self.Box.OnComponentEndOverlap`
  (params (OverlappedComponent :type "PrimitiveComponent Object Reference") (OtherActor :type "Actor Object Reference") (OtherComp :type "PrimitiveComponent Object Reference") (OtherBodyIndex :type Integer))
  ;[0.3883 0.9622 1] Door logic to open with key and find it to open
  (bind _asss_third_person_character (cast `/Game/ThirdPerson/Blueprints/SS_ThirdPersonCharacter` OtherActor))
  (set `self.SSRef` _asss_third_person_character)
  (`PrimitiveComponent.SetRenderCustomDepth` (`self.StaticMesh`) false)
  (`SceneComponent.SetVisibility` (`self.Widget`) false false)
  (set `self.canDoorOpen?` false))

(event `InputAction|ItemInteraction`
  (params (Key :type "Key Structure"))
  (:`Pressed`
    (if (`self.canDoorOpen?`)
      _)))

(fn `UserConstructionScript`)