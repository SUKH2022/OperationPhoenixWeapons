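; Base melee enemy AI character with combo attacks, hit reactions, delayed ragdoll and overhead health, assassination and investigation widgets.
; Attack feeds a CanAttack-gated montage combo that buffers input and branches on AttackIndex; Attack3 is never called.
; A looping-timer sword sphere trace and a single front trace damage "Damageable" actors with shake, sound and particles.
; Taking damage resets the combo and launches the AI along the player's facing; widgets billboard toward the camera each tick.
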(event `self.ReceiveBeginPlay`
  ;[0.05127 0.05127 0.05127] BeginPlay Configs
  (bind _aswb_dummy_health_bar (cast `` (`WidgetComponent.GetWidget` (`self.Health Bar Widget`))))
  (set `self.HealthBarUI` null _aswb_dummy_health_bar))

(event `self.ReceiveTick`
  (params (DeltaSeconds :type "Float (single-precision)"))
  ;[0.05127 0.05127 0.05127] EventTick Updates
  (`SceneComponent.K2_SetWorldRotation` (`self.Assassinate Widget`) (`KismetMathLibrary.FindLookAtRotation` (`SceneComponent.K2_GetComponentLocation` (`self.Assassinate Widget`)) (`SceneComponent.K2_GetComponentLocation` (`PlayerCameraManager.TransformComponent` (`GameplayStatics.GetPlayerCameraManager` 0)))) false false)
  (`SceneComponent.K2_SetWorldRotation` (`self.Health Bar Widget`) (`KismetMathLibrary.FindLookAtRotation` (`SceneComponent.K2_GetComponentLocation` (`self.Assassinate Widget`)) (`SceneComponent.K2_GetComponentLocation` (`PlayerCameraManager.TransformComponent` (`GameplayStatics.GetPlayerCameraManager` 0)))) false false)
  (`SceneComponent.K2_SetWorldRotation` (`self.Investigate Widget`) (`KismetMathLibrary.FindLookAtRotation` (`SceneComponent.K2_GetComponentLocation` (`self.Assassinate Widget`)) (`SceneComponent.K2_GetComponentLocation` (`PlayerCameraManager.TransformComponent` (`GameplayStatics.GetPlayerCameraManager` 0)))) false false))

(event `Ragdoll`
  ;[0.05127 0.05127 0.05127] Ragdoll
  (`|ExecutionSequence`
    (:`then_0`
      (`KismetSystemLibrary.Delay` 2.5)
      (`PrimitiveComponent.SetSimulatePhysics` (`self.Mesh`) true))
    (:`then_1`
      (`KismetSystemLibrary.Delay` 1.7)
      (`GameplayStatics.PlaySoundAtLocation` null (`self.K2_GetActorLocation`) (struct) 1.0 1.0 0.0 null null null null)
      (`SceneComponent.SetVisibility` (`self.Health Bar Widget`) false false))))

(event `self.Assassination Radius.OnComponentBeginOverlap`
  (params (OverlappedComponent :type "PrimitiveComponent Object Reference") (OtherActor :type "Actor Object Reference") (OtherComp :type "PrimitiveComponent Object Reference") (OtherBodyIndex :type Integer) (bFromSweep :type Boolean) (SweepResult :type "HitResult Structure (by ref)"))
  ;[0.05127 0.05127 0.05127] Execute Command UI
  (if (`KismetArrayLibrary.Array_Contains` (`self.Tags`) "Damageable")
    (cast `/Game/ThirdPerson/Blueprints/SS_ThirdPersonCharacter` OtherActor)
    (`SceneComponent.SetVisibility` (`self.Assassinate Widget`) true false)))

(event `self.Assassination Radius.OnComponentEndOverlap`
  (params (OverlappedComponent :type "PrimitiveComponent Object Reference") (OtherActor :type "Actor Object Reference") (OtherComp :type "PrimitiveComponent Object Reference") (OtherBodyIndex :type Integer))
  ;[0.05127 0.05127 0.05127] Execute Command UI
  (if (`KismetArrayLibrary.Array_Contains` (`self.Tags`) "Damageable")
    (cast `/Game/ThirdPerson/Blueprints/SS_ThirdPersonCharacter` OtherActor)
    (`SceneComponent.SetVisibility` (`self.Assassinate Widget`) false false)))

(event `self.ReceiveAnyDamage`
  (params (Damage :type "Float (single-precision)") (DamageType :type "DamageType Object Reference") (InstigatedBy :type "Controller Object Reference") (DamageCauser :type "Actor Object Reference"))
  (bind _hitanims (`self.hitAnims`))
  ;[0.05127 0.05127 0.05127] Damage taken and death
  (`self.Stop Combo`)
  (`self.PlayAnimMontage` (`|GetArrayItem` _hitanims (`KismetMathLibrary.RandomIntegerInRange` 0 (- (`KismetArrayLibrary.Array_Length` _hitanims) 1))))
  (bind _asss_third_person_character (cast `/Game/ThirdPerson/Blueprints/SS_ThirdPersonCharacter` (`GameplayStatics.GetPlayerCharacter` 0)))
  (`self.LaunchCharacter` (* (`KismetMathLibrary.GetForwardVector` (`self.K2_GetActorRotation` _asss_third_person_character)) 700.0))
  (`GameplayStatics.PlaySoundAtLocation` null (`self.K2_GetActorLocation`) (struct) 1.0 (`KismetMathLibrary.RandomFloatInRange` 1.0 1.3) 0.0 null null null null))

(event `Attack 1`
  ;[0.05127 0.05127 0.05127] Combo
  ;;[0.05127 0.05127 0.05127] Attack 1
  (`/Engine/EditorBlueprintResources/StandardMacros.DoOnce` false :!label _label
    (:`Completed`
      (`KismetSystemLibrary.Delay` 0.1)
      (`|PlayMontage` (`self.Mesh`) null (`self.AttackSpeed`)
        (:`then`
          (set `self.Attack Index` 1)
          (goto _label :!via `Reset`))))))

(event `Sword Attack Combo From BT`
  ;[0.05127 0.05127 0.05127] Combo
  ;;[0.05127 0.05127 0.05127] Attack Input
  (if (`self.Can Attack?`)
    (`self.Sword Attack`)))

(event `Sword Attack`
  ;[0.05127 0.05127 0.05127] Combo
  ;;[0.05127 0.05127 0.05127] Sword Attack
  (if (`self.is Attacking?`)
    (set `self.Save Attack?` true)
    (else
      (set `self.is Attacking?` true)
      (switch `int` (`self.Attack Index`) :!label _label_2
        (:`0`
          (`self.Attack 1`))
        (:`1`
          (`self.Attack 2`))
        (:`2`
          (`self.Attack 4`))))))

(event `Attack 2`
  ;[0.05127 0.05127 0.05127] Combo
  ;;[0.05127 0.05127 0.05127] Attack 2
  (`/Engine/EditorBlueprintResources/StandardMacros.DoOnce` false :!label _label_3
    (:`Completed`
      (`KismetSystemLibrary.Delay` 0.1)
      (`|PlayMontage` (`self.Mesh`) null (`self.AttackSpeed`)
        (:`then`
          (set `self.Attack Index` 2)
          (goto _label_3 :!via `Reset`))))))

(event `Sword Attack Combo`
  ;[0.05127 0.05127 0.05127] Combo
  ;;[0.05127 0.05127 0.05127] Combo Continue
  (if (`self.Save Attack?`)
    (set `self.Save Attack?` false)
    (goto _label_2)
    (else
      (`self.Stop Combo`))))

(event `Attack 3`
  ;[0.05127 0.05127 0.05127] Combo
  ;;[0.05127 0.05127 0.05127] Attack 3
  (`/Engine/EditorBlueprintResources/StandardMacros.DoOnce` false :!label _label_4
    (:`Completed`
      (`KismetSystemLibrary.Delay` 0.1)
      (`|PlayMontage` (`self.Mesh`) null (`self.AttackSpeed`)
        (:`then`
          (set `self.Attack Index` 3)
          (goto _label_4 :!via `Reset`))))))

(event `Stop Combo`
  ;[0.05127 0.05127 0.05127] Combo
  ;;[0.05127 0.05127 0.05127] Stop Combo / Attack
  (set `self.is Attacking?` false)
  (set `self.Attack Index` 0))

(event `Attack 4`
  ;[0.05127 0.05127 0.05127] Combo
  ;;[0.05127 0.05127 0.05127] Attack 4
  (`/Engine/EditorBlueprintResources/StandardMacros.DoOnce` false :!label _label_5
    (:`Completed`
      (`KismetSystemLibrary.Delay` 0.1)
      (`|PlayMontage` (`self.Mesh`) null (`self.AttackSpeed`)
        (:`then`
          (set `self.Attack Index` 4)
          (goto _label_5 :!via `Reset`))))))

(event `Start Sword Trace`
  ;[0.05127 0.05127 0.05127] Sword Trace
  (bind _returnvalue (`KismetSystemLibrary.K2_SetTimerDelegate` (delegate `Sword Trace Loop`) 0.01 true))
  (set `self.Sword Trace Loop Timer` _returnvalue))

(event `Sword Trace Loop`
  ;[0.05127 0.05127 0.05127] Sword Trace
  (bind (_outhit _returnvalue) (`KismetSystemLibrary.SphereTraceSingle` (`SceneComponent.K2_GetComponentLocation` (`self.Sword Top Point`)) (`SceneComponent.K2_GetComponentLocation` (`self.Sword Bottom Point`)) 3.0 "TraceTypeQuery1"))
  (if _returnvalue
    (bind (_bblockinghit _binitialoverlap _time _distance _location _impactpoint _normal _impactnormal _physmat _hitactor) (`GameplayStatics.BreakHitResult` _outhit))
    (if (`self.ActorHasTag` _hitactor "Damageable")
      (`KismetSystemLibrary.PrintText` "Hit!!!" true true (struct :`R` 1.0 :`G` 0.095177 :`A` 1.0))
      (`/Engine/EditorBlueprintResources/StandardMacros.DoOnce` false :!label _label_6
        (:`Completed`
          (`GameplayStatics.ApplyDamage` _hitactor 10.0)
          (`GameplayStatics.PlayWorldCameraShake` null _location 0.0 2000.0)
          (`self.Play Sword Hit Sounds`)
          (`GameplayStatics.SpawnEmitterAtLocation` null _location (`KismetMathLibrary.MakeRotFromXY` _normal _normal) (0.4 0.4 0.4) true "AutoRelease")
          (`KismetSystemLibrary.Delay` 0.5)
          (goto _label_6 :!via `Reset`))))))

(event `Stop Sword Trace`
  ;[0.05127 0.05127 0.05127] Sword Trace
  (`KismetSystemLibrary.K2_ClearAndInvalidateTimerHandle` (`self.Sword Trace Loop Timer`)))

(event `Front Player Trace`
  (bind _returnvalue (`SceneComponent.K2_GetComponentLocation` (`self.Front Trace`)))
  ;[0.05127 0.05127 0.05127] Front Trace (Stab and kick)
  (bind (_outhit _returnvalue_2) (`KismetSystemLibrary.SphereTraceSingle` _returnvalue _returnvalue 25.0 "TraceTypeQuery1"))
  (if _returnvalue_2
    (bind (_bblockinghit _binitialoverlap _time _distance _location _impactpoint _normal _impactnormal _physmat _hitactor) (`GameplayStatics.BreakHitResult` _outhit))
    (if (`self.ActorHasTag` _hitactor "Damageable")
      (`KismetSystemLibrary.PrintText` "Hit!!!" true true (struct :`R` 1.0 :`B` 0.087898 :`A` 1.0))
      (`GameplayStatics.ApplyDamage` _hitactor 10.0)
      (`GameplayStatics.PlayWorldCameraShake` null _location 0.0 2000.0)
      (`self.Play Sword Hit Sounds`)
      (`GameplayStatics.SpawnEmitterAtLocation` null _location (`KismetMathLibrary.MakeRotFromXY` _normal _normal) (0.4 0.4 0.4) true "AutoRelease"))))

(event `Play Sword Hit Sounds`
  ;[0.05127 0.05127 0.05127] Play hit sounds
  (`GameplayStatics.PlaySoundAtLocation` null (`self.K2_GetActorLocation`) (struct) 0.5 1.0 0.0 null null null null))

(event `Enable Investigation Icon`
  (`SceneComponent.SetVisibility` (`self.Investigate Widget`) true false))

(event `Disable Investigation Icon`
  (`SceneComponent.SetVisibility` (`self.Investigate Widget`) false false))

(fn `Attack`
  (returns (`Animation Duration` :type "Float (double-precision)"))
  (`self.Sword Attack Combo From BT`)
  (return 0.4))

(fn `UserConstructionScript`)