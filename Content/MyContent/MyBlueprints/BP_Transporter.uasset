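; BP_Transporter is a transporter pad that sends the player character to the level named in LevelName.
; Construction script and BeginPlay both show that name on the Level2 text.
; Capsule overlap by an SS_ThirdPersonCharacter disables movement and centers the character's mesh on the pad in X and Y.
; It then plays a swirl effect and beam-out sound, and opens the level after a short delay.
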(event `self.ReceiveBeginPlay`
  ;[1 1 1] updates text render obj to show target level
  (`TextRenderComponent.K2_SetText` (`self.Level_2`) (`KismetTextLibrary.Conv_NameToText` (`self.Level Name`))))

(event `self.Capsule.OnComponentBeginOverlap`
  (params (OverlappedComponent :type "PrimitiveComponent Object Reference") (OtherActor :type "Actor Object Reference") (OtherComp :type "PrimitiveComponent Object Reference") (OtherBodyIndex :type Integer) (bFromSweep :type Boolean) (SweepResult :type "HitResult Structure (by ref)"))
  (bind _returnvalue (`SceneComponent.K2_GetComponentLocation` OverlappedComponent))
  (bind (_returnvalue_x _returnvalue_y) (`KismetMathLibrary.BreakVector` (`SceneComponent.K2_GetComponentLocation` (`self.StaticMesh`))))
  ;[1 1 1] Health option
  (if true
    ;[1 1 1] stop the player from over running the transporter pad
    (bind _asss_third_person_character (cast `/Game/ThirdPerson/Blueprints/SS_ThirdPersonCharacter` OtherActor))
    (`CharacterMovementComponent.DisableMovement` (`Character.CharacterMovement` _asss_third_person_character))
    ;[1 1 1] center character on transporter pad
    (`SceneComponent.K2_SetWorldLocation` (`Character.Mesh` _asss_third_person_character) (`KismetMathLibrary.MakeVector` _returnvalue_x _returnvalue_y) false false)
    ;[1 1 1] Play VFX swirl and sound then open specified level
    (`NiagaraFunctionLibrary.SpawnSystemAtLocation` null _returnvalue)
    (`GameplayStatics.PlaySoundAtLocation` "/Game/MyContent/Audios/TransporterBeamOut.TransporterBeamOut" _returnvalue (struct) 1.0 1.0 0.0 null null null null)
    (`KismetSystemLibrary.Delay` 2.65)
    (`GameplayStatics.OpenLevel` (`self.Level Name`))))

(fn `UserConstructionScript`
  ;[1 1 1] displays target level name
  (`TextRenderComponent.K2_SetText` (`self.Level_2`) (`KismetTextLibrary.Conv_NameToText` (`self.Level Name`))))