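; NPC spawner actor that creates NPC_Enemy actors at its own location, up to EnemyMaxNumber in total.
; After a ten-second delay from BeginPlay, a looping timer calls SpawnNPC1 every EnemySpawnRateSecs.
; Each call increments a counter and spawns only within the limit, though the timer is never cleared.
; A sphere marker and a text label summarising count and rate, refreshed by the construction script, are hidden in game.
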(event `self.ReceiveBeginPlay`
  (`|ExecutionSequence`
    (:`then_0`
      ;[1 1 1] Wait 10 seconds and then start spawning enemies at specified rate
      (`KismetSystemLibrary.Delay` 10.0)
      (`KismetSystemLibrary.K2_SetTimer` null "SpawnNPC1" (`self.EnemySpawnRateSecs`) true))
    (:`then_1`
      ;[1 1 1] turns off sphere and text visibility in game
      (`SceneComponent.SetVisibility` (`self.SphereLocmarker`) false false)
      (`SceneComponent.SetVisibility` (`self.TextRenderNumEnemies`) false false))
    (:`then_2`
      ;[1 1 1] update text display on enemies
      (`TextRenderComponent.K2_SetText` (`self.TextRenderNumEnemies`) (`KismetTextLibrary.Conv_StringToText` (`KismetStringLibrary.Concat_StrStr` (`KismetStringLibrary.Conv_IntToString` (`self.EnemyMaxNumber`)) " enemies, 1 every " (`KismetStringLibrary.TimeSecondsToString` (`self.EnemySpawnRateSecs`)) "seconds"))))))

(fn `SpawnNPC1`
  ;[1 1 1] check max number enemies reached
  (bind _result (`/Engine/EditorBlueprintResources/StandardMacros.IncrementInt` (`self.EnemyNumber`))
    (:`  `
      (if (<= _result (`self.EnemyMaxNumber`))
        ;[1 1 1] Spawns enemy
        (`|SpawnActorFromClass` "/Game/AI_Man/NPC_Enemy.NPC_Enemy_C" (`SceneComponent.K2_GetComponentToWorld` (`self.DefaultSceneRoot`)) "Undefined" "MultiplyWithRoot" null null)))))

(fn `UserConstructionScript`
  ;[1 1 1] update text display on enemies
  (`TextRenderComponent.K2_SetText` (`self.TextRenderNumEnemies`) (`KismetTextLibrary.Conv_StringToText` (`KismetStringLibrary.Concat_StrStr` (`KismetStringLibrary.Conv_IntToString` (`self.EnemyMaxNumber`)) " enemies, 1 every " (`KismetStringLibrary.TimeSecondsToString` (`self.EnemySpawnRateSecs`)) "seconds"))))